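; BP_ShutdownButton is an interactable world button that forms part of a button-sequence puzzle checked by the game state.
; On interaction it turns its number green and glowing through a dynamic material instance, then passes itself to the game state's CheckButtonSequence.
; It binds to the game state's OnButtonSequenceFailed dispatcher, which restores the white, unlit look and resets the item.
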(event Custom|OnButtonSequenceFailed_Event
  (bind _dynamicmaterialinst (Variables|Default|GetDynamicMaterialInst))
  (Rendering|Material|SetVectorParameterValue _dynamicmaterialinst "NumberColour" "(R=1.000000,G=1.000000,B=1.000000,A=1.000000)" :!class /Script/Engine.MaterialInstanceDynamic)
  (Rendering|Material|SetScalarParameterValue _dynamicmaterialinst "Emission" 0.0 :!class /Script/Engine.MaterialInstanceDynamic)
  (Class|LI2DTriggerBase|ResetThisItem))

(event EventBeginPlay
  (bind _meshcomp (Variables|Default|GetMeshComp))
  (bind _returnvalue (Rendering|Material|CreateDynamicMaterialInstance _meshcomp 0 (Rendering|Material|GetMaterial _meshcomp 0) "None" :!class /Script/Engine.PrimitiveComponent))
  (Variables|Default|SetDynamicMaterialInst _returnvalue)
  (EventDispatchers|AssignOnButtonSequenceFailed (Variables|Default|GetGameStateRef) (delegate Custom|OnButtonSequenceFailed_Event)))

(event EventOnItemHasBeenInteractedwith
  (bind _dynamicmaterialinst (Variables|Default|GetDynamicMaterialInst))
  (Rendering|Material|SetVectorParameterValue _dynamicmaterialinst "NumberColour" "(R=0.025612,G=0.536458,B=0.027412,A=1.000000)" :!class /Script/Engine.MaterialInstanceDynamic)
  (Rendering|Material|SetScalarParameterValue _dynamicmaterialinst "Emission" 0.1 :!class /Script/Engine.MaterialInstanceDynamic)
  (Class|LI2DGameStateBase|CheckButtonSequence (Variables|Default|GetGameStateRef) self))

(fn ConstructionScript)